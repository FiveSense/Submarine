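; Missile pawn for the submarine game that flies at a target actor or fixed point and damages the Ship it hits.
; Once fired, Tick steers it by FloatingPawnMovement and look-at rotation, tracking above a live target's position.
; Actor-targeted shots take the camera from the main submarine; exploding spawns an emitter and passes it to the target Ship.
; A dynamic material's "Volume" parameter drops to zero above Z=0.
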(event OnComponentHit(StaticMesh)
  (params (HitComponent :type Primitive%20Component%20Object%20Reference) (OtherActor :type Actor%20Object%20Reference) (OtherComp :type Primitive%20Component%20Object%20Reference) (NormalImpulse :type Vector :default "0, 0, 0") (Hit :type Hit%20Result%20Structure%20%28by%20ref%29))
  ;[1 1 1] 接触爆炸 & 自动爆炸
  (bind _asship (Utilities|Casting|CastToShip OtherActor))
  (CallFunction|Explode)
  (Default|Damage _asship 1))

(event Custom|FireIt
  (params (Begin :type Vector) (End :type Vector) (Target :type Actor%20Object%20Reference))
  ;[1 1 1] 发射自身
  (Utilities|FlowControl|Sequence
    (:then_0
      (Utilities|IsValid Target
        (:Is%20Valid
          (Variables|Default|SetTargetActor Target)
          (Variables|Default|SetBeginPlace (Transformation|GetActorLocation))
          (Variables|Default|SetEndPlace (Transformation|GetActorLocation (Variables|Default|GetTargetActor)))
          (bind _assubmarine_game_mode (Utilities|Casting|CastToSubmarineGameMode (Game|GetGameMode)))
          (Default|ChangeCamera _assubmarine_game_mode "NewEnumerator1" self (Variables|/Game/Blueprints/GameFrame/SubmarineGameMode.SubmarineGameMode_C|GetMainSubmarine _assubmarine_game_mode) 0.0))
        (:Is%20Not%20Valid
          (Variables|Default|SetBeginPlace Begin)
          (Variables|Default|SetEndPlace End)
          (Variables|Default|SetTargetActor 0)
          (Variables|Default|SetisUseEndPlace true))))
    (:then_1
      (Variables|Default|SetisFire true))))

(event Custom|Explode
  ;[1 1 1] 接触爆炸 & 自动爆炸
  (bind _returnvalue (Effects|SpawnEmitteratLocation "/Game/MilitaryShipsPack/Particles/PS_ExplosionWithShrapnel.PS_ExplosionWithShrapnel" (Variables|Default|GetEndPlace)))
  (Transformation|SetWorldScale3D _returnvalue "100.000000,100.000000,100.000000")
  (bind _assubmarine_game_mode (Utilities|Casting|CastToSubmarineGameMode (Game|GetGameMode)))
  (bind _asship (Utilities|Casting|CastToShip (Variables|Default|GetTargetActor)))
  (Default|ChangeCamera _assubmarine_game_mode "NewEnumerator2" _asship self 2.0)
  (Actor|DestroyActor))

(event Collision|EventActorBeginOverlap
  (params (OtherActor :type Actor%20Object%20Reference)))

(event EventBeginPlay
  (Rendering|Material|SetScalarParameterValue (Variables|Default|GetMissileMatInstance) "Volume" 1.0 :!class /Script/Engine.MaterialInstanceDynamic)
  (if (Variables|Default|GetisTest)
    (CallFunction|FireIt "0, 0, 0" "0, 0, 0" (Variables|Default|GetTargetActor))))

(event EventTick
  (params (DeltaSeconds :type Float%20%28single-precision%29))
  (bind _floatingpawnmovement (Variables|Default|GetFloatingPawnMovement))
  (bind _targetactor (Variables|Default|GetTargetActor))
  ;[1 1 1] 发射导航
  (Utilities|FlowControl|Sequence
    (:then_0
      (if (Variables|Default|GetisFire)
        (Variables|Default|SetBeginPlace (Transformation|GetActorLocation))
        (if (Variables|Default|GetisUseEndPlace)
          _
          (else
            (Utilities|IsValid _targetactor
              (:Is%20Valid
                (Variables|Default|SetEndPlace (+ (Transformation|GetActorLocation _targetactor) "0, 0,2000.000000"))))))
        (Class|PawnMovementComponent|AddInputVector _floatingpawnmovement (Math|Rotator|GetRotationXVector (Math|Rotator|FindLookatRotation (Variables|Default|GetBeginPlace) (Variables|Default|GetEndPlace))) true)
        (Variables|/Script/Engine.FloatingPawnMovement|SetMaxSpeed _floatingpawnmovement 1e+04)
        (Transformation|SetActorRotation self (Math|Rotator|FindLookatRotation (Variables|Default|GetBeginPlace) (Variables|Default|GetEndPlace)))))
    (:then_1
      (if (> (.z (Transformation|GetActorLocation)) 0.0)
        (Rendering|Material|SetScalarParameterValue (Variables|Default|GetMissileMatInstance) "Volume" 0.0 :!class /Script/Engine.MaterialInstanceDynamic)))))

(fn ConstructionScript
  (bind _staticmesh (Variables|Default|GetStaticMesh))
  (bind _returnvalue (Rendering|Material|CreateDynamicMaterialInstance _staticmesh 0 (Rendering|Material|GetMaterial _staticmesh 0) :!class /Script/Engine.PrimitiveComponent))
  (Variables|Default|SetMissileMatInstance _returnvalue))