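; Submarine pawn that cruises automatically and descends when sunk, with the movement logic marked as a sinking test.
; Yaw and pitch axis inputs rotate the controller, while movement follows fixed world axes independent of that rotation.
; Each tick forces FloatingPawnMovement input along world +X and sets max speed, or straight down while IsSunk is true.
; The Sunk event sets that flag.
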(event Custom|Sunk
  (params (isSunk :type Boolean))
  ;[1 1 1] 沉没测试
  (Variables|Default|SetisSunk isSunk))

(event EventTick
  (params (DeltaSeconds :type Float%20%28single-precision%29))
  (bind _floatingpawnmovement (Variables|Default|GetFloatingPawnMovement))
  ;[1 1 1] 沉没测试
  (if (Variables|Default|GetisSunk)
    (Class|PawnMovementComponent|AddInputVector _floatingpawnmovement "0.000000,0.000000,-1.000000" true)
    (else
      (Class|PawnMovementComponent|AddInputVector _floatingpawnmovement "1.000000,0.000000,0.000000" true)
      (Variables|/Script/Engine.FloatingPawnMovement|SetMaxSpeed (Variables|Default|GetFloatingPawnMovement) 1.5e+03))))

(event Input|AxisEvents|InputAxisMoveRight
  (params (AxisValue :type Float%20%28single-precision%29))
  (Pawn|Input|AddControllerYawInput AxisValue))

(event Input|AxisEvents|InputAxisMoveUp
  (params (AxisValue :type Float%20%28single-precision%29))
  (Pawn|Input|AddControllerPitchInput AxisValue))

(fn ConstructionScript)