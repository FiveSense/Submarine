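; Game mode for the submarine game that switches the player's view by possessing different pawns.
; ChangeCamera takes a target type and has player controller 0 possess a missile, a ship or the submarine, then spawns a default controller for the vacated pawn.
; The ship view is temporary: after a delay, BackToSubmarine re-possesses the first SubmarinePawn found in the level and returns the ship to a default controller.
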(event Custom|ChangeCamera
  (params (NewCamera :type E_Camera%20Enum) (NewPawn :type Pawn%20Object%20Reference) (OldPawn :type Pawn%20Object%20Reference) (Delay :type Float%20%28single-precision%29))
  (bind _returnvalue (Game|GetPlayerController 0))
  (Variables|Default|SetOldTempPawn OldPawn)
  (Utilities|FlowControl|Sequence
    (:then_0
      (switch Utilities|FlowControl|Switch|SwitchonE_Camera NewCamera
        (:NewEnumerator0
          (CallFunction|BacktoSubmarine OldPawn))
        (:NewEnumerator1
          (bind _asmissile (Utilities|Casting|CastToMissile NewPawn))
          (Pawn|Possess _returnvalue _asmissile))
        (:NewEnumerator2
          (bind _astest_ship (Utilities|Casting|CastToTestShip NewPawn))
          (Pawn|Possess _returnvalue _astest_ship)
          (Variables|Default|SetOldTempPawn _astest_ship)
          (Utilities|FlowControl|Delay Delay)
          (CallFunction|BacktoSubmarine _astest_ship))))
    (:then_1
      (Pawn|SpawnDefaultController OldPawn))))

(event Custom|BackToSubmarine
  (params (OldPawn :type Pawn%20Object%20Reference))
  (bind _outactors (Actor|GetAllActorsOfClass "/Game/Blueprints/GameFrame/SubmarinePawn.SubmarinePawn_C"))
  (Pawn|Possess (Game|GetPlayerController 0) (Utilities|Array|Get(acopy) _outactors))
  (Pawn|SpawnDefaultController OldPawn))

(event EventBeginPlay)

(event EventTick
  (params (DeltaSeconds :type Float%20%28single-precision%29)))

(fn ConstructionScript)